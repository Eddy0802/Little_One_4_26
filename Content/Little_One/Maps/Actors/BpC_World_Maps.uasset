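; World map component that defines the playable map area from two corner actors, TopLeft and BottomRight, and converts world locations into map coordinates.
; Height comes from the corners' distance along world X and width from their distance along world Y.
; Location conversion returns absolute offsets from TopLeft with axes swapped, so world Y becomes map X, without normalizing to map size.
; InitializeMaps stores a valid Player reference or prints an error.
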(event Custom|InitializeMaps
  (params (Player :type Character%20Object%20Reference))
  (Utilities|IsValid Player
    (:Is%20Valid
      (Variables|Default|SetPlayer Player))
    (:Is%20Not%20Valid
      (Development|PrintString "error player is not valid" true true "(R=1.000000,G=0.000000,B=0.028129,A=1.000000)" 5.0))))

(event EventBeginPlay)

(event EventTick
  (params (DeltaSeconds :type Float%20%28single-precision%29)))

(fn GetMapsHeight
  (return (Math|Float|Absolute(Float) (- (.X (Math|Vector|BreakVector (Transformation|GetActorLocation (Variables|Settings|GetBottom_Right)))) (.X (Math|Vector|BreakVector (Transformation|GetActorLocation (Variables|settings|GetTop_Left))))))))

(fn GetMapsWidth
  (return (Math|Float|Absolute(Float) (- (.Y (Math|Vector|BreakVector (Transformation|GetActorLocation (Variables|Settings|GetBottom_Right)))) (.Y (Math|Vector|BreakVector (Transformation|GetActorLocation (Variables|settings|GetTop_Left))))))))

(fn ConvertLocationtoMapLocation
  (params (Location :type Vector))
  (bind (_x _y) (Math|Vector|BreakVector Location))
  (bind _top_left (Variables|settings|GetTop_Left))
  (bind _returnvalue (Transformation|GetActorLocation _top_left))
  (bind (_x_2 _y_2) (Math|Vector|BreakVector _returnvalue))
  (return (Math|Vector2D|MakeVector2D (Math|Float|Absolute(Float) (- _y _y_2)) (Math|Float|Absolute(Float) (- _x _x_2)))))